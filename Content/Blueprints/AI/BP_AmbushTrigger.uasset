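; Ambush trigger volume that drops hidden assassins from ceiling spawn points when the player enters it.
; On BeginPlay it spawns an "Ambush"-tagged BP_Assassin at each "SpawnCeiling"-tagged actor, hidden with movement mode None.
; When a BP_ThirdPersonCharacter with WaveCount 1 overlaps the Box, it unhides them and switches movement to Falling.
; A Triggered flag makes the ambush fire only once.
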(event OnComponentBeginOverlap(Box)
  (params (OverlappedComponent :type Primitive%20Component%20Object%20Reference) (OtherActor :type Actor%20Object%20Reference) (OtherComp :type Primitive%20Component%20Object%20Reference) (OtherBodyIndex :type Integer) (bFromSweep :type Boolean) (SweepResult :type Hit%20Result%20Structure%20%28by%20ref%29))
  (if (not (Variables|Default|GetbTriggered))
    (bind _asbp_third_person_character (Utilities|Casting|CastToBP_ThirdPersonCharacter OtherActor))
    (if (== (Variables|/Script/VaultView.VaultViewCharacter|GetWaveCount _asbp_third_person_character) 1)
      (for _array_element (Variables|Default|GetHiddenAssassins)
        (Rendering|SetActorHiddenInGame _array_element false)
        (Pawn|Components|CharacterMovement|SetMovementMode (Variables|/Script/Engine.Character|GetCharacterMovement _array_element) "MOVE_Falling" 0))
      (Variables|Default|SetbTriggered true))))

(event EventBeginPlay
  (bind _outactors (Actor|GetAllActorswithTag "SpawnCeiling"))
  (for _array_element _outactors
    (bind _returnvalue (Game|SpawnActorfromClass "/Game/Blueprints/AI/BP_Assassin.BP_Assassin_C" (Transformation|GetActorTransform _array_element) "AlwaysSpawn" "MultiplyWithRoot" 0 0))
    (Utilities|Array|Add (Variables|/Script/Engine.Actor|GetTags _returnvalue) "Ambush")
    (Pawn|Components|CharacterMovement|SetMovementMode (Variables|/Script/Engine.Character|GetCharacterMovement _returnvalue) "MOVE_None" 0)
    (Rendering|SetActorHiddenInGame _returnvalue true)
    (Utilities|Array|Add (Variables|Default|GetHiddenAssassins) _returnvalue)))

(event Collision|EventActorBeginOverlap
  (params (OtherActor :type Actor%20Object%20Reference)))

(event EventTick
  (params (DeltaSeconds :type Float%20%28single-precision%29)))

(fn ConstructionScript)